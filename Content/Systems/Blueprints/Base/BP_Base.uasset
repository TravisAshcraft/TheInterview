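; BP_Base is a base actor with a child-actor shape and a text counter, providing helpers for color assignment and count display.
; SetBaseColor gives a target one of five random color material instances, while CheckAndSetColor copies the BP_Base_Shape child's material onto a passed mesh when they differ.
; SetCounterToCurrentNumber writes the count to the TextRender, which Tick holds at zero world rotation pending camera alignment.
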(event `self.ReceiveTick`
  (params (DeltaSeconds :type "Float (single-precision)"))
  ;[1 1 1] todo set text to line up with camera
  (`SceneComponent.K2_SetWorldRotation` :`self` (`self.TextRender`)))

(fn `CheckAndSetColor`
  (params (ActorStaticMesh1 :type "StaticMeshComponent Object Reference"))
  (locals (BaseColor :type "MaterialInterface Object Reference") (ActorStaticMesh :type "StaticMeshComponent Object Reference"))
  ;[1 1 1] checks to see if the actor is of the same color if not then it sets its color to the corresponding color
  (bind _asbp_base_shape (cast `/Game/Systems/Blueprints/Base/BP_Base_Shape` (`ChildActorComponent.ChildActor` (`self.CA_Base_Shape`))))
  (bind _returnvalue (`PrimitiveComponent.GetMaterial` (`/Game/Systems/Blueprints/Base/BP_Base_Shape.SM_Base_Shape` _asbp_base_shape) 0))
  (set `local.BaseColor` _returnvalue)
  (if (not (== (`PrimitiveComponent.GetMaterial` (`local.ActorStaticMesh1`) 0) _returnvalue))
    (`PrimitiveComponent.SetMaterial` (`local.ActorStaticMesh1`) 0 (`local.BaseColor`))))

(fn `SetBaseColor`
  (params (Target :type "PrimitiveComponent Object Reference"))
  ;[1 1 1] Sets the colors for the bases
  (`PrimitiveComponent.SetMaterial` Target 0 (select `int` (`KismetMathLibrary.RandomIntegerInRange` 0 4) :`0` "/Game/Assets/Meshes/Actors/Materials/MI_Green.MI_Green" :`1` "/Game/Assets/Meshes/Actors/Materials/MI_Blue.MI_Blue" :`2` "/Game/Assets/Meshes/Actors/Materials/MI_Red.MI_Red" :`3` "/Game/Assets/Meshes/Actors/Materials/MI_Purple.MI_Purple" :`4` "/Game/Assets/Meshes/Actors/Materials/MI_Black.MI_Black" :!type "MaterialInterface Object Reference")))

(fn `SetCounterToCurrentNumber`
  (params (NumberOf :type Integer))
  ;[1 1 1] Sets the counter to the corresponding number
  (`TextRenderComponent.K2_SetText` (`self.TextRender`) (`KismetTextLibrary.Conv_IntToText` NumberOf)))

(fn `UserConstructionScript`)