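; BPC_Base_Cube is a base that counts BP_ActorCube actors inside its Box trigger and manages their color.
; BeginPlay initializes the counter and passes the CABaseShape child mesh to SetBaseColor.
; Begin overlap increments and displays the count, then runs CheckAndSetColor on the entering cube's mesh.
; End overlap decrements it and applies the leaving cube's CurrentMaterial to the mesh captured at begin overlap, which may belong to another cube.
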(event `self.ReceiveTick`
  (params (DeltaSeconds :type "Float (single-precision)")))

(event `self.ReceiveBeginPlay`
  ;[1 1 1] Sets the counter to zero
  (`self.SetCounterToCurrentNumber` (`self.CountOfCubes`))
  ;[1 1 1] Checks to see if the color is equal if not sets the actors color equal to base
  (bind _asstatic_mesh_component (cast `StaticMeshComponent` (`SceneComponent.GetChildComponent` (`self.CA_Base_Shape`) 0)))
  (`self.SetBaseColor` _asstatic_mesh_component))

(event `self.Box.OnComponentBeginOverlap`
  (params (OverlappedComponent :type "PrimitiveComponent Object Reference") (OtherActor :type "Actor Object Reference") (OtherComp :type "PrimitiveComponent Object Reference") (OtherBodyIndex :type Integer) (bFromSweep :type Boolean) (SweepResult :type "HitResult Structure (by ref)"))
  (bind _asbp_actor_cube (cast `/Game/Systems/Blueprints/Actors/BP_ActorCube` OtherActor))
  (set `self.ActorStaticMesh_0` (`/Game/Systems/Blueprints/Actors/BP_ActorBaseClass.StaticMesh` _asbp_actor_cube))
  ;[1 1 1] Adds one to the count
  (bind _result (`/Engine/EditorBlueprintResources/StandardMacros.IncrementInt` (`self.CountOfCubes`))
    (:`  `
      (bind _output_get (set `self.CountOfCubes` _result))
      (`self.SetCounterToCurrentNumber` _output_get)
      (`self.CheckAndSetColor` (`self.ActorStaticMesh_0`)))))

(event `self.Box.OnComponentEndOverlap`
  (params (OverlappedComponent :type "PrimitiveComponent Object Reference") (OtherActor :type "Actor Object Reference") (OtherComp :type "PrimitiveComponent Object Reference") (OtherBodyIndex :type Integer))
  (bind _asbp_actor_cube (cast `/Game/Systems/Blueprints/Actors/BP_ActorCube` OtherActor))
  ;[1 1 1] Takes one from the count
  (bind _result (`/Engine/EditorBlueprintResources/StandardMacros.DecrementInt` (`self.CountOfCubes`))
    (:`  `
      (bind _output_get (set `self.CountOfCubes` _result))
      (`self.SetCounterToCurrentNumber` _output_get)
      (`PrimitiveComponent.SetMaterial` (`self.ActorStaticMesh_0`) 0 (`/Game/Systems/Blueprints/Actors/BP_ActorBaseClass.CurrentMaterial` _asbp_actor_cube)))))

(fn `UserConstructionScript`
  (`parent.UserConstructionScript`))