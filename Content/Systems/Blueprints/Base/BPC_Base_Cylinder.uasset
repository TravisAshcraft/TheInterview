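; A base zone Blueprint that keeps a live count of cylinder actors inside its box volume and displays it on a text render.
; Box begin and end overlap events, filtered by a cast to BP_CylinderActor, increment and decrement CountOfCylinders.
; The text is set from the count on BeginPlay and refreshed after each change, so Tick does no work.
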(event `self.ReceiveTick`
  (params (DeltaSeconds :type "Float (single-precision)")))

(event `self.ReceiveBeginPlay`
  (`TextRenderComponent.K2_SetText` (`self.TextRender`) (`KismetTextLibrary.Conv_IntToText` (`self.CountOfCylinders`))))

(event `self.Box.OnComponentBeginOverlap`
  (params (OverlappedComponent :type "PrimitiveComponent Object Reference") (OtherActor :type "Actor Object Reference") (OtherComp :type "PrimitiveComponent Object Reference") (OtherBodyIndex :type Integer) (bFromSweep :type Boolean) (SweepResult :type "HitResult Structure (by ref)"))
  (cast `/Game/Systems/Blueprints/Actors/BP_CylinderActor` OtherActor)
  (bind _result (`/Engine/EditorBlueprintResources/StandardMacros.IncrementInt` (`self.CountOfCylinders`))
    (:`  `
      (bind _output_get (set `self.CountOfCylinders` _result))
      (`TextRenderComponent.K2_SetText` (`self.TextRender`) (`KismetTextLibrary.Conv_IntToText` _output_get)))))

(event `self.Box.OnComponentEndOverlap`
  (params (OverlappedComponent :type "PrimitiveComponent Object Reference") (OtherActor :type "Actor Object Reference") (OtherComp :type "PrimitiveComponent Object Reference") (OtherBodyIndex :type Integer))
  (cast `/Game/Systems/Blueprints/Actors/BP_CylinderActor` OtherActor)
  (bind _result (`/Engine/EditorBlueprintResources/StandardMacros.DecrementInt` (`self.CountOfCylinders`))
    (:`  `
      (bind _output_get (set `self.CountOfCylinders` _result))
      (`TextRenderComponent.K2_SetText` (`self.TextRender`) (`KismetTextLibrary.Conv_IntToText` _output_get)))))

(fn `UserConstructionScript`
  (`parent.UserConstructionScript`))