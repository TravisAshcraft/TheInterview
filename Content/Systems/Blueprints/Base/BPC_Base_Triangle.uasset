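; Triangle base Blueprint that counts BP_TriangleActors inside its box and recolors them to the base color.
; BeginPlay initializes the counter display and applies the base color to its child shape mesh.
; Begin overlap increments the count and runs CheckAndSetColor on the entering mesh.
; End overlap decrements it and applies the leaving actor's CurrentMaterial, though to the mesh reference taken from the begin-overlap cast.
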(event `self.ReceiveBeginPlay`
  (`self.SetCounterToCurrentNumber` (`self.CountOfTriangles`))
  ;[1 1 1] Checks to see if the color is equal if not sets the actors color equal to base
  (bind _asstatic_mesh_component (cast `StaticMeshComponent` (`SceneComponent.GetChildComponent` (`self.CA_Base_Shape`) 0)))
  (`self.SetBaseColor` _asstatic_mesh_component))

(event `self.Box.OnComponentBeginOverlap`
  (params (OverlappedComponent :type "PrimitiveComponent Object Reference") (OtherActor :type "Actor Object Reference") (OtherComp :type "PrimitiveComponent Object Reference") (OtherBodyIndex :type Integer) (bFromSweep :type Boolean) (SweepResult :type "HitResult Structure (by ref)"))
  (bind _asbp_triangle_actor (cast `/Game/Systems/Blueprints/Actors/BP_TriangleActor` OtherActor))
  (set `self.Static Mesh` (`/Game/Systems/Blueprints/Actors/BP_ActorBaseClass.StaticMesh` _asbp_triangle_actor))
  ;[1 1 1] Adds one to count
  (bind _result (`/Engine/EditorBlueprintResources/StandardMacros.IncrementInt` (`self.CountOfTriangles`))
    (:`  `
      (bind _output_get (set `self.CountOfTriangles` _result))
      (`self.SetCounterToCurrentNumber` _output_get)
      ;[1 1 1] Sets actor color to base color
      (`self.CheckAndSetColor` (`self.Static Mesh`)))))

(event `self.Box.OnComponentEndOverlap`
  (params (OverlappedComponent :type "PrimitiveComponent Object Reference") (OtherActor :type "Actor Object Reference") (OtherComp :type "PrimitiveComponent Object Reference") (OtherBodyIndex :type Integer))
  (bind _asbp_triangle_actor (cast `/Game/Systems/Blueprints/Actors/BP_TriangleActor` OtherActor))
  ;[1 1 1] Takes one away
  (bind _result (`/Engine/EditorBlueprintResources/StandardMacros.DecrementInt` (`self.CountOfTriangles`))
    (:`  `
      (bind _output_get (set `self.CountOfTriangles` _result))
      (`self.SetCounterToCurrentNumber` _output_get)
      ;[1 1 1] Sets material back to original material
      (`PrimitiveComponent.SetMaterial` (`self.Static Mesh`) 0 (`/Game/Systems/Blueprints/Actors/BP_ActorBaseClass.CurrentMaterial` _asbp_triangle_actor)))))

(fn `UserConstructionScript`
  (`parent.UserConstructionScript`))