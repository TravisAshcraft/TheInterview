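; BP_ShapeSpawner is a spawner actor that places a random shape, or nothing, at its own location.
; On BeginPlay it sets its ChildActor component's class to a random pick of cube, cylinder, sphere, triangle or an empty option.
; CheckIfSpawnedOrNot then sets DidSpawn according to whether that child actor class is empty.
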(event `self.ReceiveBeginPlay`
  ;[1 1 1] Randomly selects which actor to spawn in this actors location
  (`ChildActorComponent.SetChildActorClass` (`self.ChildActor`) (select `int` (`KismetMathLibrary.RandomIntegerInRange` 0 4) :`0` "/Game/Systems/Blueprints/Actors/BP_ActorCube.BP_ActorCube_C" :`1` "/Game/Systems/Blueprints/Actors/BP_CylinderActor.BP_CylinderActor_C" :`2` "/Game/Systems/Blueprints/Actors/BP_SphereActor.BP_SphereActor_C" :`3` "/Game/Systems/Blueprints/Actors/BP_TriangleActor.BP_TriangleActor_C" :`4` null :!type "Actor Class Reference"))
  (`self.CheckIfSpawnedOrNot`))

(fn `CheckIfSpawnedOrNot`
  ;[1 1 1] Checks to see if child actor class is empty or not.
  (if (!= (`ChildActorComponent.ChildActorClass` (`self.ChildActor`)) null)
    (set `self.DidSpawn` true)
    (else
      (set `self.DidSpawn` false))))

(fn `UserConstructionScript`)