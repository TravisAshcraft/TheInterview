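; Player controller for a free camera with mouse-driven actor placement.
; Axis input moves the pawn locally at a spring-arm-scaled speed with a fast modifier; screen-edge scrolling runs when neither moving nor panning.
; Holding Pan hides the cursor and opens gates for mouse rotation with clamped pitch.
; Tick polls every BP_ActorBaseClass, snapping clicked ones to the cursor trace; left click in placement mode drops the actor, despite the SpawnActor name.
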(event `self.ReceiveBeginPlay`
  ;[1 1 1] Event Begin Play
  (set `self.bShowMouseCursor` true))

(event `InputAction|MoveFaster`
  (params (Key :type "Key Structure"))
  ;[1 1 1] Move Faster
  (:`Pressed`
    (set `self.FastMoveMultiplier` 2.0))
  (:`Released`
    (set `self.FastMoveMultiplier` 1.0)))

(event `InputAxis|MoveRight`
  (params (AxisValue :type "Float (single-precision)"))
  ;[1 1 1] Movement on the Y-axis
  (if (> AxisValue 0.0)
    (set `self.IsMoving?` true)
    (bind _returnvalue (`self.MovementY` (* AxisValue (* (`self.MovementSpeedCalculation`) (`self.FastMoveMultiplier`))) :!label _label))
    (`self.K2_SetActorTransform` (`self.GetPlayerRef`) _returnvalue false false)
    (elif (< AxisValue 0.0)
      (goto _label)
      (else
        (set `self.IsMoving?` false)))))

(event `InputAxis|MoveForward`
  (params (AxisValue :type "Float (single-precision)"))
  ;[1 1 1] Movement on the X-axis
  (if (> AxisValue 0.0)
    (set `self.IsMoving?` true)
    (bind _returnvalue (`self.MovementX` (* AxisValue (* (`self.MovementSpeedCalculation`) (`self.FastMoveMultiplier`))) :!label _label_2))
    (`self.K2_SetActorTransform` (`self.GetPlayerRef`) _returnvalue false false)
    (elif (< AxisValue 0.0)
      (goto _label_2)
      (else
        (set `self.IsMoving?` false)))))

(event `InputAxisKey|MouseX`
  (params (AxisValue :type "Float (single-precision)"))
  ;[1 1 1] Allows the playe to move with the mouse on the edge of the screen if no other action going on.
  (if (not (or (`self.IsInPan?`) (`self.IsMoving?`)))
    (bind (_xspeed_multiplied_ _yspeed_multiplied_) (`self.ScreenEdgeMovement` :!label _label_3))
    (`self.K2_AddActorLocalOffset` (`self.GetPlayerRef`) (`KismetMathLibrary.MakeVector` _xspeed_multiplied_ _yspeed_multiplied_) true false)))

(event `InputAxisKey|MouseY`
  (params (AxisValue :type "Float (single-precision)"))
  ;[1 1 1] Allows the playe to move with the mouse on the edge of the screen if no other action going on.
  (if (not (or (`self.IsInPan?`) (`self.IsMoving?`)))
    (goto _label_3 :!via `MouseYExec`)))

(event `self.ReceiveTick`
  (params (DeltaSeconds :type "Float (single-precision)"))
  (`|ExecutionSequence`
    (:`then_0`
      (bind _outactors (`GameplayStatics.GetAllActorsOfClass` "/Game/Systems/Blueprints/Actors/BP_ActorBaseClass.BP_ActorBaseClass_C"))
      (for _array_element _outactors
        (bind _isclicked (`/Game/Systems/Blueprints/Interfaces/INT_ActorBase.GetIsClicked` _array_element))
        (if _isclicked
          (bind _output_get (set `self.ActorBaseClassRef` _array_element))
          (bind _output_get_2 (set `self.PlaceableActor` _output_get))
          (set `self.PlaceableActorType` (`GameplayStatics.GetObjectClass` _output_get_2))
          (`self.UpdatePlacement`))))))

(event `InputAxisKey|MouseX`
  (params (AxisValue :type "Float (single-precision)"))
  ;[1 1 1] Pan X
  (`/Engine/EditorBlueprintResources/StandardMacros.Gate` true :!label _label_4
    (:`Exit`
      (`self.K2_SetActorRotation` (`self.GetPlayerRef`) (`KismetMathLibrary.MakeRotator` (.roll (`self.K2_GetActorRotation` (`self.GetPlayerRef`))) (.pitch (`self.K2_GetActorRotation` (`self.GetPlayerRef`))) (+ (.yaw (`self.K2_GetActorRotation` (`self.GetPlayerRef`))) (* (`self.PanSenitivity`) AxisValue))) false))))

(event `Key|LeftMouseButton`
  (params (Key :type "Key Structure"))
  (:`Pressed`
    (if (stale `/Game/Systems/Blueprints/Interfaces/INT_PlayerController.SetPlacementMode` _output_get)
      (`self.SpawnActor` (`self.ActorBaseClassRef`)))))

(event `InputAction|Pan`
  (params (Key :type "Key Structure"))
  ;[1 1 1] Pan X
  (:`Pressed`
    (set `self.IsInPan?` true)
    (`self.ShowMouseCursor` false)
    (goto _label_4 :!via `Open`))
  (:`Released`
    (set `self.IsInPan?` false)
    (`self.ShowMouseCursor` true)
    (goto _label_4 :!via `Close`)))

(event `/Game/Systems/Blueprints/Interfaces/INT_PlayerController.SetPlacementMode`
  (params (PlacementMode :type Boolean))
  (bind _output_get (set `self.PlacementModeEnabled` PlacementMode)))

(event `InputAxisKey|MouseY`
  (params (AxisValue :type "Float (single-precision)"))
  (bind (_returnvalue_roll _returnvalue_pitch _returnvalue_yaw) (`KismetMathLibrary.BreakRotator` (`KismetMathLibrary.MakeRotator` (.roll (`self.K2_GetActorRotation` (`self.GetPlayerRef`))) (+ (.pitch (`self.K2_GetActorRotation` (`self.GetPlayerRef`))) (* (`self.PanSenitivity`) AxisValue)) (.yaw (`self.K2_GetActorRotation` (`self.GetPlayerRef`))))))
  ;[1 1 1] Pan Y
  (`/Engine/EditorBlueprintResources/StandardMacros.Gate` true :!label _label_5
    (:`Exit`
      (`self.K2_SetActorRotation` (`self.GetPlayerRef`) (`KismetMathLibrary.MakeRotator` _returnvalue_roll (`KismetMathLibrary.FClamp` _returnvalue_pitch -40.0 80.0) _returnvalue_yaw) false))))

(event `InputAction|Pan`
  (params (Key :type "Key Structure"))
  ;[1 1 1] Pan Y
  (:`Pressed`
    (set `self.IsInPan?` true)
    (`self.ShowMouseCursor` false)
    (goto _label_5 :!via `Open`))
  (:`Released`
    (set `self.IsInPan?` false)
    (`self.ShowMouseCursor` true)
    (goto _label_5 :!via `Close`)))

(fn `GetPlayerRef`
  (returns (PlayerRef :type "Actor Object Reference"))
  (bind _playerref (message `/Game/Systems/Blueprints/Interfaces/INT_PlayerPawn.GetPlayerRef` (`GameplayStatics.GetPlayerPawn` 0)))
  (return _playerref))

(fn `MovementSpeedCalculation`
  (returns (MoveSensitivity :type "Float (double-precision)"))
  (bind _springarm (message `/Game/Systems/Blueprints/Interfaces/INT_PlayerPawn.GetCameraSpringArm` (`GameplayStatics.GetPlayerPawn` 0)))
  (return (`KismetMathLibrary.FClamp` (/ (`SpringArmComponent.TargetArmLength` _springarm) 100.0) 5.0 20.0)))

(fn `SetPlacementModeEnabled`
  (params (`IsPlacementEnabled?` :type Boolean))
  (if (== `IsPlacementEnabled?` (`self.PlacementModeEnabled`))
    (return)
    (else
      (bind _output_get (set `self.PlacementModeEnabled` `IsPlacementEnabled?`))
      (if _output_get
        (`AddComponent|NODE_AddBP_MoveActorComponent-0`)
        (else
          (set `self.PlacementModeEnabled` false))))))

(fn `SpawnActor`
  (params (Target :type "/Game/Systems/Blueprints/Actors/BP_ActorBaseClass Object Reference"))
  (`/Engine/EditorBlueprintResources/StandardMacros.IsValid` (`self.PlaceableActor`)
    (:`Is Valid`
      (`self.SetPlacementModeEnabled` false)
      (`/Game/Systems/Blueprints/Gameplay/BP_ClickableComponet.SetIsClicked` (`/Game/Systems/Blueprints/Actors/BP_ActorBaseClass.BP_ClickableComponet` Target) false))))

(fn `UpdatePlacement`
  (bind (_worldlocation _worlddirection) (`self.DeprojectMousePositionToWorld`))
  (bind _placeableactor (`self.PlaceableActor`))
  (bind _outhit (`KismetSystemLibrary.LineTraceSingle` _worldlocation (+ _worldlocation (* _worlddirection 1000000.0)) "TraceTypeQuery3"))
  (bind (_bblockinghit _binitialoverlap _time _distance _location) (`GameplayStatics.BreakHitResult` _outhit))
  (if _bblockinghit
    (`/Engine/EditorBlueprintResources/StandardMacros.IsValid` _placeableactor
      (:`Is Valid`
        (`self.K2_SetActorLocation` _placeableactor _location false false)))))

(fn `UserConstructionScript`)