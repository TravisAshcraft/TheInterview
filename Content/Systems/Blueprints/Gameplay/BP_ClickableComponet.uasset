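; BP_ClickableComponet is a component that makes its owning actor clickable and flags it visually under the mouse cursor.
; On BeginPlay it caches the owner's static mesh and, only if one exists, binds the owner's cursor-over and click events.
; Hovering toggles the mesh's render custom depth.
; Clicking sets IsClicked, resettable through SetIsClicked, and calls SetPlacementModeMessage on the player controller.
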(event `self.ReceiveBeginPlay`
  (bind _returnvalue (`self.GetOwner`))
  (bind _returnvalue_2 (`Actor.GetComponentByClass` _returnvalue "/Script/Engine.StaticMeshComponent"))
  ;[1 1 1] Checks to see if clicked actor has a static mesh if true then it saves the static mesh to variable
  (`/Engine/EditorBlueprintResources/StandardMacros.IsValid` _returnvalue_2
    (:`Is Valid`
      (set `self.StaticMeshComponent` _returnvalue_2)
      ;[1 1 1] Sets the render depth to true when mouse is over actor
      (add `Actor.OnBeginCursorOver` _returnvalue (delegate `Event_MouseOver`))
      ;[1 1 1] Sets the render depth to false when mouse is not over actor
      (add `Actor.OnEndCursorOver` _returnvalue (delegate `Event_MouseOverEnd`))
      (add `Actor.OnClicked` _returnvalue (delegate `Event_OnClicked`)))))

(event `Event_MouseOverEnd`
  (params (TouchedActor :type "Actor Object Reference"))
  (bind _staticmeshcomponent (`self.StaticMeshComponent`))
  ;[1 1 1] Sets the render depth to false when mouse is not over actor
  (`/Engine/EditorBlueprintResources/StandardMacros.IsValid` _staticmeshcomponent
    (:`Is Valid`
      (`PrimitiveComponent.SetRenderCustomDepth` _staticmeshcomponent false))))

(event `Event_OnClicked`
  (params (TouchedActor :type "Actor Object Reference") (ButtonPressed :type "Key Structure"))
  (set `self.IsClicked?` true)
  (message `/Game/Systems/Blueprints/Interfaces/INT_PlayerController.SetPlacementMode` (`GameplayStatics.GetPlayerController` 0) true))

(event `Event_MouseOver`
  (params (TouchedActor :type "Actor Object Reference"))
  (bind _staticmeshcomponent (`self.StaticMeshComponent`))
  ;[1 1 1] Sets the render depth to true when mouse is over actor
  (`/Engine/EditorBlueprintResources/StandardMacros.IsValid` _staticmeshcomponent
    (:`Is Valid`
      (`PrimitiveComponent.SetRenderCustomDepth` _staticmeshcomponent true))))

(fn `SetIsClicked`
  (params (NewParam :type Boolean))
  (set `self.IsClicked?` NewParam))