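; Base actor class that snaps itself to the ground and exposes a clicked state.
; On BeginPlay, it traces straight down for a single object type and teleport-free moves to the hit location, without sweeping or checking that the trace hit.
; GetIsClicked passes through the IsClicked flag from its clickable component.
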(event `self.ReceiveBeginPlay`
  (bind (_returnvalue_x _returnvalue_y _returnvalue_z) (`KismetMathLibrary.BreakVector` (`self.K2_GetActorLocation`)))
  ;[1 1 1] Sets and keeps the actor on the ground
  (bind _outhit (`KismetSystemLibrary.LineTraceSingleForObjects` (`self.K2_GetActorLocation`) (`KismetMathLibrary.MakeVector` _returnvalue_x _returnvalue_y (+ _returnvalue_z -1000.0)) (`|MakeArray` "ObjectTypeQuery7" :!type "EObjectTypeQuery Enum")))
  (`self.K2_SetActorLocation` (`.Location` (`GameplayStatics.BreakHitResult` _outhit))))

(fn `GetIsClicked`
  (returns (IsClicked :type Boolean))
  (return (`/Game/Systems/Blueprints/Gameplay/BP_ClickableComponet.IsClicked?` (`self.BP_ClickableComponet`))))

(fn `UserConstructionScript`)